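; BP_OldPalCharacter is a character Blueprint assembled from modular skeletal mesh parts.
; Its construction script sets BodyComp as the leader pose for the Feet, Torso and Legs meshes, so they follow the body's animation.
; The helper EnableMasterPose links only parts with a valid mesh and neither a post-process AnimBlueprint nor their own anim class.
; The event graph holds no gameplay logic.
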(fn `EnableMasterPose`
  (params (SkeletalMeshComponent :type "SkeletalMeshComponent Object Reference"))
  (bind _skeletalmeshasset (`SkeletalMeshComponent.SkeletalMeshAsset` SkeletalMeshComponent))
  (if (`KismetSystemLibrary.IsValid` _skeletalmeshasset)
    (if (not (or (`KismetSystemLibrary.IsValidClass` (`SkeletalMesh.PostProcessAnimBlueprint` _skeletalmeshasset)) (`KismetSystemLibrary.IsValidClass` (`SkeletalMeshComponent.AnimClass` SkeletalMeshComponent))))
      (`SkinnedMeshComponent.SetLeaderPoseComponent` SkeletalMeshComponent (`self.bodyComp`) false false))))

(fn `UserConstructionScript`
  (`self.EnableMasterPose` (`self.Feet`))
  (`self.EnableMasterPose` (`self.Torso`))
  (`self.EnableMasterPose` (`self.Legs`)))