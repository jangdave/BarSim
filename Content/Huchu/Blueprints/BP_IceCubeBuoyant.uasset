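; BP_IceCubeBuoyant is an ice cube actor that starts drifting upward when its box component is hit, suggesting buoyancy.
; Each hit on BoxComp destroys any existing ProjectileMovement component and adds a new one with low capped speed, negative gravity scale and upward velocity.
; The hit also prints a debug string, while BeginPlay, Tick, overlap and leftover setter chains do nothing.
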(event `self.ReceiveBeginPlay`)

(event `self.boxComp.OnComponentHit`
  (params (HitComponent :type "PrimitiveComponent Object Reference") (OtherActor :type "Actor Object Reference") (OtherComp :type "PrimitiveComponent Object Reference") (NormalImpulse :type "Vector Structure") (Hit :type "HitResult Structure (by ref)"))
  (`/Engine/EditorBlueprintResources/StandardMacros.IsValid` (`self.ProjectileMovement`)
    (:`Is Valid`
      (`ActorComponent.K2_DestroyComponent` (`self.ProjectileMovement`)))
    (:`Is Not Valid`
      _))
  (bind _returnvalue (`AddComponent|NODE_AddProjectileMovementComponent-1`))
  (bind _output_get (set `self.ProjectileMovement` _returnvalue))
  (set `ProjectileMovementComponent.InitialSpeed` 9.0 _output_get)
  (set `ProjectileMovementComponent.MaxSpeed` 9.0 _output_get)
  (set `ProjectileMovementComponent.ProjectileGravityScale` -1.0 _output_get)
  (set `MovementComponent.Velocity` (0.0 0.0 1.0) _output_get)
  (`KismetSystemLibrary.PrintString` "Hello"))

(fn `UserConstructionScript`)