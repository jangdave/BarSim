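; BP_MixingGlass1 is a mixing glass that registers stirring with a bar spoon.
; Two sphere triggers feed the same logic when a BarSpoon begins overlapping either one, provided the glass is at least a tenth full.
; Each accepted overlap toggles StirStarted through a shared FlipFlop, increases StirRate and resets TimePassed.
; This graph only writes that stir state and has no active Tick logic to consume it.
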(event `self.Sphere.OnComponentBeginOverlap`
  (params (OverlappedComponent :type "PrimitiveComponent Object Reference") (OtherActor :type "Actor Object Reference") (OtherComp :type "PrimitiveComponent Object Reference") (OtherBodyIndex :type Integer) (bFromSweep :type Boolean) (SweepResult :type "HitResult Structure (by ref)"))
  (cast `BarSpoon` OtherActor)
  (if (>= (/ (`self.contents`) (`self.cupSize`)) 0.1) :!label _label
    (`/Engine/EditorBlueprintResources/StandardMacros.FlipFlop`
      (:`A`
        (set `self.bStirStarted` true))
      (:`B`
        (set `self.bStirStarted` false)))
    (set `self.stirRate` (+ (`self.stirRate`) 0.5))
    (set `self.timePassed` 0.0)))

(event `self.Sphere1.OnComponentBeginOverlap`
  (params (OverlappedComponent :type "PrimitiveComponent Object Reference") (OtherActor :type "Actor Object Reference") (OtherComp :type "PrimitiveComponent Object Reference") (OtherBodyIndex :type Integer) (bFromSweep :type Boolean) (SweepResult :type "HitResult Structure (by ref)"))
  (cast `BarSpoon` OtherActor)
  (goto _label))

(fn `UserConstructionScript`)