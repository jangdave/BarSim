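; BP_RockGlass is a rock glass that plays a clank sound when it hits another CupBase actor.
; Its CupComp hit event checks the other cup's clank audio component to avoid overlapping sounds from one collision.
; It spawns the clank at the impact point with slightly randomized high pitch and stores the audio component.
; A DoOnce with a short delayed reset throttles repeated hits.
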(event `self.cupComp.OnComponentHit`
  (params (HitComponent :type "PrimitiveComponent Object Reference") (OtherActor :type "Actor Object Reference") (OtherComp :type "PrimitiveComponent Object Reference") (NormalImpulse :type "Vector Structure") (Hit :type "HitResult Structure (by ref)"))
  (bind _ascup_base (cast `CupBase` OtherActor))
  (bind _glassclankaudiocomp (`CupBase.glassClankAudioComp` _ascup_base))
  (`/Engine/EditorBlueprintResources/StandardMacros.IsValid` _glassclankaudiocomp
    (:`Is Valid`
      (`/Engine/EditorBlueprintResources/StandardMacros.DoOnce` false
        (:`Completed`
          (if (not (`AudioComponent.IsPlaying` _glassclankaudiocomp))
            (bind _returnvalue (`GameplayStatics.SpawnSoundAtLocation` "/Game/KHJContents/Sounds/BottleClank/GlassClank.GlassClank" (`.Location` (`GameplayStatics.BreakHitResult` Hit)) (struct) 0.5 (`KismetMathLibrary.RandomFloatInRange` 1.6 1.7) 0.0 null null :!label _label))
            (set `self.glassClankAudioComp` _returnvalue)
            (`KismetSystemLibrary.Delay` 0.1)
            (goto _label_2 :!via `Reset`)))))
    (:`Is Not Valid`
      (`/Engine/EditorBlueprintResources/StandardMacros.DoOnce` false :!label _label_2
        (:`Completed`
          (goto _label))))))

(fn `UserConstructionScript`)