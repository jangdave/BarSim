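; White rum bottle Blueprint that drives a liquid material to show agitation from movement and the amount remaining.
; Each Tick derives acceleration from an offset, rotation-aware point on the mesh, smoothing it with slower fadeout at low speed.
; Remains sets liquid level plus piecewise-linear side and upside-down correction coefficients, with negative values pushing the level far down.
; Construction creates the dynamic material with a random starting level, which Tick then overrides.
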(event `self.ReceiveTick`
  (params (DeltaSeconds :type "Float (single-precision)"))
  (bind _meshcomp (`self.meshComp`))
  (bind (_maxacceleration_x _maxacceleration_y) (`KismetMathLibrary.BreakVector2D` (`self.MaxAcceleration`)))
  (bind (_maxacceleration_x_2 _maxacceleration_y_2) (`KismetMathLibrary.BreakVector2D` (`self.MaxAcceleration`)))
  (bind _liquidlevel (`self.LiquidLevel`))
  (bind _liquidlevel_2 (`self.LiquidLevel`))
  (bind _returnvalue (- (* (`self.remains`) 0.0315) 0.1))
  ;[0.04971 0.1248 0] Calculate Bottle Acceleration
  ;;[0.04184 0.2195 0.003] Get current bottle position with offset
  ;; (to account for angular velocity changes)
  (set `self.CurrentPosition` (+ (`SceneComponent.K2_GetComponentLocation` _meshcomp) (`KismetMathLibrary.GreaterGreater_VectorRotator` (`KismetMathLibrary.Conv_DoubleToVector` (`self.PosOffset`)) (`SceneComponent.K2_GetComponentRotation` _meshcomp))))
  ;;[0.1124 0.3427 0] Calculate velocity using bottle's last and current position
  (set `self.Velocity` (/ (- (`self.CurrentPosition`) (`self.LastPosition`)) (`GameplayStatics.GetWorldDeltaSeconds`)))
  ;;[0.21 0.5385 0] Calculate acceleration using bottle's last and current velocity
  (set `self.Acceleration` (`KismetMathLibrary.ClampVectorSize` (`KismetMathLibrary.VInterpTo` (`self.Acceleration`) (`KismetMathLibrary.Vector_GetAbs` (- (`self.Velocity`) (`self.LastVelocity`))) (`GameplayStatics.GetWorldDeltaSeconds`) (`KismetMathLibrary.SelectFloat` 20.0 0.5 (> (`KismetMathLibrary.VSize` (`self.Velocity`)) 25.0))) _maxacceleration_x_2 _maxacceleration_y_2))
  ;;[0.3107 0.7969 0] Pass acceleration into bottle's material
  (`MaterialInstanceDynamic.SetVectorParameterValue` (`self.BottleDynamicMat`) "BottleAcceleration" (`KismetMathLibrary.Conv_VectorToLinearColor` (/ (`self.Acceleration`) _maxacceleration_y)))
  ;;[0.4494 1 0] Cache last Velocity and Position
  (set `self.LastVelocity` (`self.Velocity`))
  (set `self.LastPosition` (`self.CurrentPosition`))
  (if (< (`self.remains`) 0.0)
    (`MaterialInstanceDynamic.SetScalarParameterValue` (`self.BottleDynamicMat`) "LiquidLevel" -100.0)
    (else
      (`MaterialInstanceDynamic.SetScalarParameterValue` (`self.BottleDynamicMat`) "LiquidLevel" _returnvalue)
      (set `self.LiquidLevel` _returnvalue)
      (if (<= (`self.LiquidLevel`) 0.1)
        (`MaterialInstanceDynamic.SetScalarParameterValue` (`self.BottleDynamicMat`) "LiquidLevelSideCoef" (+ (* (`self.LiquidLevel`) -2.0) 0.7))
        (else
          (`MaterialInstanceDynamic.SetScalarParameterValue` (`self.BottleDynamicMat`) "LiquidLevelSideCoef" (+ (* (`self.LiquidLevel`) -0.5) 0.55))))
      (if (and (<= _liquidlevel 0.7) (<= 0.5 _liquidlevel))
        (`MaterialInstanceDynamic.SetScalarParameterValue` (`self.BottleDynamicMat`) "LiquidLevelUpsideDownCoef" (+ (* (`self.LiquidLevel`) -0.6) 1.7))
        (elif (and (<= _liquidlevel_2 0.5) (<= 0.35 _liquidlevel_2))
          (`MaterialInstanceDynamic.SetScalarParameterValue` (`self.BottleDynamicMat`) "LiquidLevelUpsideDownCoef" (+ (* (`self.LiquidLevel`) -0.67) 1.73))
          (elif (<= (`self.LiquidLevel`) 0.35)
            (`MaterialInstanceDynamic.SetScalarParameterValue` (`self.BottleDynamicMat`) "LiquidLevelUpsideDownCoef" (+ (* (`self.LiquidLevel`) -6.8) 3.88))))))))

(fn `UserConstructionScript`
  (bind _posoffset (`self.posOffset`))
  (bind _meshcomp (`self.meshComp`))
  (bind _returnvalue (+ (`SceneComponent.K2_GetComponentLocation` _meshcomp) (`KismetMathLibrary.GreaterGreater_VectorRotator` (`KismetMathLibrary.MakeVector` _posoffset _posoffset _posoffset) (`SceneComponent.K2_GetComponentRotation` _meshcomp))))
  ;[1 1 1] Cache bottle's position (with rotated offset to account for angular velocity changes)
  (set `self.LastPosition` _returnvalue)
  (set `self.CurrentPosition` _returnvalue)
  ;[1 1 1] Create Dynamic Material Instance
  (bind _returnvalue_2 (`PrimitiveComponent.CreateDynamicMaterialInstance` (`self.meshComp`) 0 (`self.Source Material`) "None"))
  (set `self.BottleDynamicMat` _returnvalue_2)
  ;[1 1 1] Assign slightly random liquid level value
  (`MaterialInstanceDynamic.SetScalarParameterValue` (`self.BottleDynamicMat`) "LiquidLevel" (`KismetMathLibrary.RandomFloatInRange` 0.55 0.75)))