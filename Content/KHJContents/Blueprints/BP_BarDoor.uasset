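; Replicated, grippable VR physics door with two lever handles, a deadbolt and a key.
; The server hands lever grips on to the door and tracks Gripped, Closed and Locked.
; While held, the door simulates and ignores pawns; after release, a timeline waits for zero velocity, restores blocking and checks closure against a detached child actor's orientation.
; Optionally, Locked/Closed RepNotifies adjust constraint swing limits instead of blocking locked-door grips.
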(event `SetPlayerCollision`
  (params (Collide :type Boolean) (Simulation :type Boolean))
  ;[1 1 1] Door collision ON/OFF - called from grip/grip release
  (`PrimitiveComponent.SetSimulatePhysics` (`self.Door`) Simulation)
  (`self.SetCollision` Collide))

(event `self.ReceiveBeginPlay`
  ;[1 1 1] Begin Play - detach child actor to prevent door swing
  (`self.K2_DetachFromActor` (`ChildActorComponent.ChildActor` (`self.ChildActor`)) "KeepWorld" "KeepWorld" "KeepWorld") ; This is because otherwise it will swing with the door\nCan do this with two totally seperate actors instead but I wanted it all in one blueprint for now\n\nThe door has to be root now because otherwise it doesn't replicate
  (`/Engine/EditorBlueprintResources/ActorMacros.Switch Has Authority`
    (:`Authority`
      (bind _asdoor_key (cast `/Game/VRE/Grippables/Misc/Examples/Door/DoorKey` (`ChildActorComponent.ChildActor` (`self.ChildActor1`))))
      (set `/Game/VRE/Grippables/Misc/Examples/Door/DoorKey.OwningKeyCore` (`self.KeyCore`) _asdoor_key)
      (set `/Game/VRE/Grippables/Misc/Examples/Door/DoorKey.OwningKeyCollider` (`self.KeyCollider`) _asdoor_key)
      (`/Game/VRE/Grippables/Misc/Examples/Door/DoorKey.InitKey` _asdoor_key)
      (`GrippableStaticMeshComponent.SetDenyGripping` (`self.Door`) false))))

(event `SetCollision`
  (params (Collide :type Boolean))
  (bind _door (`self.Door`))
  ;[1 1 1] Multicast - have all connected update door collision
  (if Collide
    (`PrimitiveComponent.SetCollisionResponseToChannel` _door "ECC_Pawn" "ECR_Block") ; Block pawns from going through door
    (else
      (`PrimitiveComponent.SetCollisionResponseToChannel` _door "ECC_Pawn" "ECR_Ignore") ; Allow pawns through the door
    )))

(event `VRGripInterface.OnChildGrip`
  (params (GrippingController :type "GripMotionControllerComponent Object Reference") (GripInformation :type "BPActorGripInformation Structure (by ref)"))
  ;[1 1 1] On Child Grip (BPI call) - server sets door collision OFF and turns simulation ON
  (if (== (`.GrippedObject` (break `BPActorGripInformation` GripInformation)) (`self.Door`))
    (`/Engine/EditorBlueprintResources/ActorMacros.Switch Has Authority`
      (:`Authority`
        (`self.SetPlayerCollision` false true)
        (set `self.Gripped` true)
        (set `self.Closed` false)))))

(event `VRGripInterface.OnChildGripRelease`
  (params (ReleasingController :type "GripMotionControllerComponent Object Reference") (GripInformation :type "BPActorGripInformation Structure (by ref)") (bWasSocketed :type Boolean))
  ;[1 1 1] On Child Grip Release (BPI call) - check door velocity and change collision/simulation
  (if (== (`.GrippedObject` (break `BPActorGripInformation` GripInformation)) (`self.Door`))
    (`/Engine/EditorBlueprintResources/ActorMacros.Switch Has Authority`
      (:`Authority`
        (`Timeline|DoorStop` :!via `PlayFromStart` :!label _label
          (:`Update`
            ;;[1 1 1] If Door is not moving, set collision ON and simulation OFF
            (if (== (`SceneComponent.GetComponentVelocity` (`self.Door`)) (0.0 0.0 0.0))
              (`self.SetPlayerCollision` true)
              ;;[1 1 1] Decide on turning on/off the door gripping itself
              (`|ExecutionSequence`
                (:`then_0`
                  (goto _label :!via `Stop`))
                (:`then_1`
                  (if (== (`SceneComponent.GetRightVector` (`self.Door`)) (`self.GetActorRightVector` (`ChildActorComponent.ChildActor` (`self.ChildActor`))) :`ErrorTolerance` 0.01)
                    (set `self.Gripped` false)
                    (`GrippableStaticMeshComponent.SetDenyGripping` (`self.Door`) false)
                    (set `self.Closed` true)))))))))))

(event `self.DoorHandleLever.HandleGripped`
  (params (RefToSelf :type "/Game/VRE/Grippables/Misc/Examples/Door/DoorHandleLever Object Reference"))
  (`self.HandleDoorGrip` RefToSelf true))

(event `HandleDoorGrip`
  (params (CallingHandle :type "/Game/VRE/Grippables/Misc/Examples/Door/DoorHandleLever Object Reference") (GrippedReq :type Boolean))
  (bind _door (`self.Door`))
  ;[1 1 1] Auto grip door if the handle is gripped or if the handle is unlocked
  (`/Engine/EditorBlueprintResources/ActorMacros.Switch Has Authority`
    (:`Authority`
      (if (`self.SetAngleWhenLocked`)
        (bind (_holdingcontrollers _bisheld) (`VRGripInterface.IsHeld` CallingHandle :!label _label_2))
        (if _bisheld
          (bind _output_holdingcontroller (break `BPGripPair` (`|GetArrayItem` _holdingcontrollers)))
          (if (not (`GripMotionControllerComponent.GetIsComponentHeld` _output_holdingcontroller _door))
            (`GrippableStaticMeshComponent.SetDenyGripping` (`self.Door`) false)
            (`KismetSystemLibrary.Delay` 0.0)
            (`GripMotionControllerComponent.GripObjectByInterface` _output_holdingcontroller _door (`SceneComponent.K2_GetComponentToWorld` _door) false "None" "None" true)
            (set `self.Closed` false)))
        (elif (and (== (`self.Gripped`) GrippedReq) (not (and (`self.Locked`) (`self.Closed`))))
          (goto _label_2))))))

(event `self.DoorHandleLever2.HandleGripped`
  (params (RefToSelf :type "/Game/VRE/Grippables/Misc/Examples/Door/DoorHandleLever Object Reference"))
  (`self.HandleDoorGrip` RefToSelf true))

(event `self.DoorHandleLever.HandleUnlocked`
  (params (RefToSelf :type "/Game/VRE/Grippables/Misc/Examples/Door/DoorHandleLever Object Reference"))
  (`self.HandleDoorGrip` RefToSelf))

(event `self.DoorHandleLever2.HandleUnlocked`
  (params (RefToSelf :type "/Game/VRE/Grippables/Misc/Examples/Door/DoorHandleLever Object Reference"))
  (`self.HandleDoorGrip` RefToSelf))

(event `self.DoorHandleLever2.HandleReleased`
  (params (RefToSelf :type "/Game/VRE/Grippables/Misc/Examples/Door/DoorHandleLever Object Reference") (ReleasingHand :type "GripMotionControllerComponent Object Reference"))
  (`self.DropDoorIfHeld` ReleasingHand))

(event `self.DoorHandleLever.HandleReleased`
  (params (RefToSelf :type "/Game/VRE/Grippables/Misc/Examples/Door/DoorHandleLever Object Reference") (ReleasingHand :type "GripMotionControllerComponent Object Reference"))
  (`self.DropDoorIfHeld` ReleasingHand))

(event `self.DeadBolt.DeadboltLockState`
  (params (IsLocked :type Boolean))
  (`/Engine/EditorBlueprintResources/ActorMacros.Switch Has Authority`
    (:`Authority`
      (set `self.Locked` IsLocked))))

(fn `AdvancedGripSettings`
  (returns (ReturnValue :type "BPAdvGripSettings Structure"))
  (return))

(fn `AllowsMultipleGrips`
  (returns (ReturnValue :type Boolean))
  (return false))

(fn `ClosestGripSlotInRange`
  (params (WorldLocation :type "Vector Structure") (bSecondarySlot :type Boolean) (CallingController :type "GripMotionControllerComponent Object Reference") (OverridePrefix :type Name))
  (returns (bHadSlotInRange :type Boolean) (SlotWorldTransform :type "Transform Structure") (SlotName :type Name))
  (return false (struct) "None"))

(fn `DenyGripping`
  (params (GripInitiator :type "GripMotionControllerComponent Object Reference"))
  (returns (ReturnValue :type Boolean))
  (return true))

(fn `DropDoorIfHeld`
  (params (HoldingHand :type "GripMotionControllerComponent Object Reference"))
  (bind _door (`self.Door`))
  (`/Engine/EditorBlueprintResources/ActorMacros.Switch Has Authority`
    (:`Authority`
      (if (`GripMotionControllerComponent.GetIsObjectHeld` HoldingHand _door)
        (`GripMotionControllerComponent.DropObjectByInterface` HoldingHand _door 0 (0.0 0.0 0.0) (0.0 0.0 0.0)))
      (return))))

(fn `GetGripScripts`
  (returns (ArrayReference :type "Array of VRGripScriptBase Object Reference") (ReturnValue :type Boolean))
  (return _ false))

(fn `GetGripStiffnessAndDamping`
  (returns (GripStiffnessOut :type "Float (single-precision)") (GripDampingOut :type "Float (single-precision)"))
  (return 0.0 0.0))

(fn `GetPrimaryGripType`
  (params (bIsSlot :type Boolean))
  (returns (ReturnValue :type "EGripCollisionType Enum"))
  (return "InteractiveCollisionWithPhysics"))

(fn `GripBreakDistance`
  (returns (ReturnValue :type "Float (single-precision)"))
  (return 0.0))

(fn `GripLateUpdateSetting`
  (returns (ReturnValue :type "EGripLateUpdateSettings Enum"))
  (return "LateUpdatesAlwaysOn"))

(fn `GripMovementReplicationType`
  (returns (ReturnValue :type "EGripMovementReplicationSettings Enum"))
  (return "KeepOriginalMovement"))

(fn `IsHeld`
  (returns (HoldingControllers :type "Array of BPGripPair Structure") (bIsHeld :type Boolean))
  (return _ false))

(fn `OnRep_Closed`
  (`self.SetAngle`))

(fn `OnRep_Locked`
  (`self.SetAngle`))

(fn `RequestsSocketing`
  (returns (ParentToSocketTo :type "SceneComponent Object Reference") (OptionalSocketName :type Name) (RelativeTransform :type "Transform_NetQuantize Structure") (ReturnValue :type Boolean))
  (return null "None" (struct) false))

(fn `SecondaryGripType`
  (returns (ReturnValue :type "ESecondaryGripType Enum"))
  (return "SG_None"))

(fn `SetAngle`
  (bind _vrephysicsconstraint (`self.VREPhysicsConstraint`))
  (bind _locked (`self.Locked`))
  (bind _returnvalue (`VREPhysicsConstraintComponent.GetAngularOffset` _vrephysicsconstraint))
  (if (`self.SetAngleWhenLocked`)
    (if (and (`self.Closed`) _locked)
      (if (!= _returnvalue (struct :`Yaw` -1.0))
        (`VREPhysicsConstraintComponent.SetAngularOffset` _vrephysicsconstraint (struct :`Yaw` -1.0))
        (`PhysicsConstraintComponent.SetAngularSwing1Limit` _vrephysicsconstraint "ACM_Free" 1.0))
      (elif _locked
        _
        (elif (!= _returnvalue (struct :`Yaw` -45.0))
          (`VREPhysicsConstraintComponent.SetAngularOffset` _vrephysicsconstraint (struct :`Yaw` -45.0))
          (`PhysicsConstraintComponent.SetAngularSwing1Limit` _vrephysicsconstraint "ACM_Free" 45.0))))))

(fn `SimulateOnDrop`
  (returns (ReturnValue :type Boolean))
  (return false))

(fn `TeleportBehavior`
  (returns (ReturnValue :type "EGripInterfaceTeleportBehavior Enum"))
  (return "TeleportAllComponents"))

(fn `UserConstructionScript`)